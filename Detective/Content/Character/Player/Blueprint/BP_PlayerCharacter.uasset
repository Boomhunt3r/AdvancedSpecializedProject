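; Player character for a detective game, creating the HUD, tutorial, logbook, post-it and murder board widgets and handling logbook, pause, interact and cooldown-limited Detective View input.
; In grab mode, mouse traces pick suspects, open post-its for reading or grab them, with Tick dragging them within the board's collision box.
; Tick also compares echo IDs to set two door flags, only printing messages.
; Key 4 loads a save, restoring position, post-its and logbook entries.
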(event `self.ReceiveBeginPlay`
  (bind _mesh (`self.Mesh`))
  (`|ExecutionSequence`
    (:`then_0`
      (`SkeletalMeshComponent.SetMorphTarget` _mesh "UpperSlimming" 1.0 true))
    (:`then_1`
      (`SkeletalMeshComponent.SetMorphTarget` _mesh "ArmSlimming" 1.0 true))
    (:`then_2`
      (bind _returnvalue (`GameplayStatics.GetActorOfClass` "/Game/Gameplay/Interact/MurderBoard/Blueprint/BP_MurderBoard.BP_MurderBoard_C"))
      (set `self.MurderBoard` _returnvalue))
    (:`then_3`
      (bind _returnvalue_2 (`|CreateWidget` "/Game/UI/MainHUD/Widget_MainHUD.Widget_MainHUD_C"))
      (bind _output_get (set `self.MainHUD` _returnvalue_2))
      (`UserWidget.AddToViewport` _output_get 0))
    (:`then_4`
      (bind _returnvalue_3 (`|CreateWidget` "/Game/UI/Tutorial/WidgetTutorial.WidgetTutorial_C"))
      (bind _output_get_2 (set `self.Tutorial` _returnvalue_3))
      (`UserWidget.AddToViewport` _output_get_2 0)
      (`Widget.SetVisibility` _output_get_2 "Visible")
      (`self.LockInput`))
    (:`then_5`
      (bind _returnvalue_4 (`|CreateWidget` "/Game/UI/Logbook/BP_LogbookV2.BP_LogbookV2_C"))
      (bind _output_get_3 (set `self.LogbookV2` _returnvalue_4))
      (`self.SetLogbook` _output_get_3)
      (`UserWidget.AddToViewport` _returnvalue_4 0))
    (:`then_6`
      (bind _returnvalue_5 (`|CreateWidget` "/Game/UI/MurderBoard/Widget_PoastIt.Widget_PoastIt_C"))
      (bind _output_get_4 (set `self.PostItWidget` _returnvalue_5))
      (`UserWidget.AddToViewport` _output_get_4 0)
      (`Widget.SetVisibility` _output_get_4 "Hidden")
      (bind _outactors (`GameplayStatics.GetAllActorsOfClassWithTag` "/Script/Detective.DetectiveView" "View"))
      (set `self.DetectiveViews` _outactors))
    (:`then_7`
      (bind _returnvalue_6 (`|CreateWidget` "/Game/UI/MurderBoard/BP_MurderBoardUI.BP_MurderBoardUI_C"))
      (bind _output_get_5 (set `self.MurderUI` _returnvalue_6))
      (`UserWidget.AddToViewport` _output_get_5 0)
      (`Widget.SetVisibility` _output_get_5 "Hidden"))))

(event `self.ReceiveTick`
  (params (DeltaSeconds :type "Float (single-precision)"))
  (bind (_worldlocation _worlddirection) (`PlayerController.DeprojectMousePositionToWorld` (`GameplayStatics.GetPlayerController` 0)))
  (bind _collisionbox1 (`/Game/Gameplay/Interact/MurderBoard/Blueprint/BP_MurderBoard.CollisionBox1` (`self.MurderBoard`)))
  (bind _returnvalue_x (`KismetMathLibrary.BreakVector` (`SceneComponent.K2_GetComponentLocation` (`/Game/Gameplay/Interact/MurderBoard/Blueprint/BP_MurderBoard.MurderBoard` (`self.MurderBoard`)))))
  (bind (_returnvalue_x_2 _returnvalue_y _returnvalue_z) (`KismetMathLibrary.BreakVector` (`SceneComponent.K2_GetComponentLocation` _collisionbox1)))
  (bind (_returnvalue_x_3 _returnvalue_y_2 _returnvalue_z_2) (`KismetMathLibrary.BreakVector` (`BoxComponent.GetScaledBoxExtent` _collisionbox1)))
  (bind (_returnvalue_x_4 _returnvalue_y_3 _returnvalue_z_3) (`KismetMathLibrary.BreakVector` (+ (`KismetMathLibrary.MakeVector` (.x _worldlocation) (.y _worldlocation) (.z _worldlocation)) (* _worlddirection (`self.OriginalDistancetoObject`)))))
  ;[1 1 1] Movement and Rotation
  (if (not (`self.LogbookVisible`))
    (`|ExecutionSequence`
      (:`then_0`
        ;[1 1 1] Moving Postits
        (if (`self.Grabmode`)
          (`/Engine/EditorBlueprintResources/StandardMacros.IsValid` (`self.GrabbedComponent`)
            (:`Is Valid`
              ;[1 1 1] Check if position is in border
              (if (>= (+ _returnvalue_z _returnvalue_z_2) _returnvalue_z_3)
                (if (<= (- _returnvalue_z _returnvalue_z_2) _returnvalue_z_3)
                  (if (>= (+ _returnvalue_y _returnvalue_x_3) _returnvalue_y_3)
                    (if (<= (- _returnvalue_y _returnvalue_x_3) _returnvalue_y_3)
                      ;[1 1 1] Location Update Postits
                      (`self.K2_SetActorLocation` (`self.GrabbedComponent`) (`KismetMathLibrary.MakeVector` _returnvalue_x _returnvalue_y_3 _returnvalue_z_3) false false)))))))))
      (:`then_1`
        (set `self.Count` 0)
        (if (`self.isFirstDoorActivated`)
          (if (not (`self.isSecondDoorActivated`))
            ;[1 1 1] For Second Door
            (for _index (range (`KismetArrayLibrary.Array_Length` (`self.EchoArray`)))
              (bind _output (`|GetArrayItem` (`self.EchoArray`) _index))
              (bind _idecho (`/Game/Gameplay/Interact/Echos/BP_Hint_Base.idEcho` _output))
              (if (> _idecho (`self.EchosForFirstDoor`))
                (if (== _idecho (`/Game/Gameplay/Interact/Echos/BP_Hint_Base.idFromPlayer` _output))
                  (bind _result (`/Engine/EditorBlueprintResources/StandardMacros.IncrementInt` (`self.Count`))
                    (:`  `
                      (set `self.Count` _result))))))
            (if (== (`self.Count`) (- (`self.EchosForSecondDoor`) (`self.EchosForFirstDoor`)))
              (set `self.isSecondDoorActivated` true)
              (`KismetSystemLibrary.PrintString` "Second Door Opened")))
          (else
            ;[1 1 1] For First Echos
            (for _index_2 (range (`KismetArrayLibrary.Array_Length` (`self.EchoArray`)))
              (bind _output_2 (`|GetArrayItem` (`self.EchoArray`) _index_2))
              (bind _idecho_2 (`/Game/Gameplay/Interact/Echos/BP_Hint_Base.idEcho` _output_2))
              (if (<= _idecho_2 (`self.EchosForFirstDoor`))
                (if (> _idecho_2 0)
                  (if (== _idecho_2 (`/Game/Gameplay/Interact/Echos/BP_Hint_Base.idFromPlayer` _output_2))
                    (bind _result_2 (`/Engine/EditorBlueprintResources/StandardMacros.IncrementInt` (`self.Count`))
                      (:`  `
                        (set `self.Count` _result_2)))))))
            (if (== (`self.Count`) (`self.EchosForFirstDoor`))
              (set `self.isFirstDoorActivated` true)
              (`KismetSystemLibrary.PrintString` "Open Door"))))))))

(event `InputAction|ShowHideLogbook`
  (params (Key :type "Key Structure"))
  (bind _mainhud (`self.MainHUD`))
  ;[1 1 1] Activate Logbook
  (:`Pressed`
    (if (not (`self.Grabmode`))
      (bind _output_get (set `self.LogbookVisible` (not (`self.LogbookVisible`))))
      (`self.ShowHideLogbook` _output_get)
      (`/Engine/EditorBlueprintResources/StandardMacros.FlipFlop`
        (:`A`
          (`Widget.SetVisibility` _mainhud "Hidden"))
        (:`B`
          (`Widget.SetVisibility` _mainhud "Visible"))))))

(event `InputAction|DetectiveView`
  (params (Key :type "Key Structure"))
  (bind _mainhud (`self.MainHUD`))
  ;[1 1 1] Activate DV
  (:`Pressed`
    (if (not (`self.isDVCooldown`))
      (`self.ActivateView` (`self.DetectiveViews`))
      (set `self.isDVCooldown` true)
      (`/Game/UI/MainHUD/Widget_MainHUD.ViewHasCooldown` _mainhud)
      (`KismetSystemLibrary.Delay` 3.0)
      (`/Game/UI/MainHUD/Widget_MainHUD.ViewNoCooldown` _mainhud)
      (set `self.isDVCooldown` false)))
  (:`Released`
    (`/Engine/EditorBlueprintResources/StandardMacros.DoOnce` false
      (:`Completed`
        (`/Game/UI/MainHUD/Widget_MainHUD.DeactivateViewHint` _mainhud)))))

(event `Key|LeftMouseButton`
  (params (Key :type "Key Structure"))
  (bind _grabmode (`self.Grabmode`))
  (bind (_worldlocation _worlddirection) (`PlayerController.DeprojectMousePositionToWorld` (`GameplayStatics.GetPlayerController` 0)))
  ;[1 1 1] Moving Postits
  (:`Pressed`
    (if (`self.Pressed`)
      (if _grabmode
        (set `self.GrabbedComponent` null)
        (`PhysicsHandleComponent.ReleaseComponent` (`self.PhysicsHandle`))
        (set `self.Pressed` false))
      (else
        (set `self.Pressed` true)
        (if _grabmode
          (bind (_outhit _returnvalue) (`KismetSystemLibrary.LineTraceSingle` :`Start` _worldlocation :`End` (+ _worldlocation (* _worlddirection 10000.0)) :`TraceChannel` "TraceTypeQuery1" :`DrawDebugType` "ForDuration"))
          (if _returnvalue
            (bind (_bblockinghit _binitialoverlap _time _distance _location _impactpoint _normal _impactnormal _physmat _hitactor _hitcomponent) (`GameplayStatics.BreakHitResult` _outhit))
            ;;[1 1 1] checks if object is MOVABLE
            (if (== (`SceneComponent.Mobility` _hitcomponent) (enumliteral `EComponentMobility` "Movable"))
              (set `self.OriginalDistancetoObject` _distance)
              (set `self.GrabbedComponent` _hitactor)
              (bind (_bblockinghit_2 _binitialoverlap_2 _time_2 _distance_2 _location_2 _impactpoint_2 _normal_2 _impactnormal_2 _physmat_2 _hitactor_2 _hitcomponent_2) (`GameplayStatics.BreakHitResult` _outhit))
              (set `self.RelativeGrabLocation` (`KismetMathLibrary.InverseTransformLocation` (`KismetMathLibrary.Conv_VectorToTransform` (`self.K2_GetActorLocation` _hitactor)) _location_2))
              (elif (`ActorComponent.ComponentHasTag` _hitcomponent_2 "Suspect")
                (`Widget.SetVisibility` (`self.MurderUI`) "Visible")
                (set `/Game/UI/MurderBoard/BP_MurderBoardUI.ChosenSuspect` (`KismetSystemLibrary.GetDisplayName` _hitcomponent_2) (`self.MurderUI`))))))))))

(event `InputAction|Interact`
  (params (Key :type "Key Structure"))
  ;[1 1 1] Interaction
  (:`Pressed`
    (`self.Interact`)))

(event `Key|RightMouseButton`
  (params (Key :type "Key Structure"))
  (bind _allpostits (`self.AllPostIts`))
  (bind (_worldlocation _worlddirection) (`PlayerController.DeprojectMousePositionToWorld` (`GameplayStatics.GetPlayerController` 0)))
  (:`Pressed`
    (if (`self.Grabmode`)
      (if (not (`self.ReadPostItActive`))
        (bind _outhit (`KismetSystemLibrary.LineTraceSingle` :`Start` _worldlocation :`End` (+ _worldlocation (* _worlddirection 10000.0)) :`TraceChannel` "TraceTypeQuery1" :`DrawDebugType` "ForDuration"))
        (bind _keys (`BlueprintMapLibrary.Map_Keys` _allpostits))
        (bind _values (`BlueprintMapLibrary.Map_Values` _allpostits))
        (bind _returnvalue (`GameplayStatics.GetObjectClass` (`.HitActor` (`GameplayStatics.BreakHitResult` _outhit))))
        (if (`KismetArrayLibrary.Array_Contains` _values _returnvalue)
          (`/Game/UI/MurderBoard/Widget_PoastIt.ReadPostIt_Event` (`self.PostItWidget`) (`KismetArrayLibrary.Array_Find` _keys (`KismetArrayLibrary.Array_Find` _values _returnvalue)))
          (set `self.ReadPostItActive` true))
        (else
          (`Widget.SetVisibility` (`self.PostItWidget`) "Hidden")
          (set `self.ReadPostItActive` false))))))

(event `Key|Four`
  (params (Key :type "Key Structure"))
  (:`Pressed`
    (bind _returnvalue (`GameplayStatics.DoesSaveGameExist` "test"))
    (if _returnvalue
      (bind _returnvalue_2 (`GameplayStatics.LoadGameFromSlot` "test"))
      (bind _asbp_game_save (cast `/Game/Save/BP_GameSave` _returnvalue_2))
      (bind _output_get (set `self.Player_Location` (`/Game/Save/BP_GameSave.Player_Location` _asbp_game_save)))
      (`self.K2_SetActorLocation` _output_get)
      (bind _values (`BlueprintMapLibrary.Map_Values` (`/Game/Save/BP_GameSave.PostItsLocations` _asbp_game_save)))
      (if (> (`KismetArrayLibrary.Array_Length` _values) 0)
        (bind _postitslocations (`/Game/Save/BP_GameSave.PostItsLocations` _asbp_game_save))
        (bind _values_2 (`BlueprintMapLibrary.Map_Values` _postitslocations))
        (bind _keys (`BlueprintMapLibrary.Map_Keys` _postitslocations))
        (for (_array_element _array_index) _keys
          (`|SpawnActorFromClass` (`GameplayStatics.GetObjectClass` _array_element) (`KismetMathLibrary.MakeTransform` (`|GetArrayItem` _values_2 _array_index)) "Undefined" "OverrideRootScale" null null))
        (bind _logbookentries (`/Game/Save/BP_GameSave.LogbookEntries` _asbp_game_save))
        (bind _values_3 (`BlueprintMapLibrary.Map_Values` _logbookentries))
        (if (> (`KismetArrayLibrary.Array_Length` _values_3) 0)
          (bind _keys_2 (`BlueprintMapLibrary.Map_Keys` _logbookentries))
          (bind _values_4 (`BlueprintMapLibrary.Map_Values` _logbookentries))
          (for (_array_element_2 _array_index_2) _keys_2
            (`self.AddImageLogbookEntry` _array_element_2 (`|GetArrayItem` _values_4 _array_index_2))))
        (else
          (bind _values_5 (`BlueprintMapLibrary.Map_Values` (`/Game/Save/BP_GameSave.LogbookEntries` _asbp_game_save)))
          (if (> (`KismetArrayLibrary.Array_Length` _values_5) 0)
            (bind _keys_3 (`BlueprintMapLibrary.Map_Keys` _logbookentries))
            (bind _values_6 (`BlueprintMapLibrary.Map_Values` _logbookentries))
            (for (_array_element_3 _array_index_3) _keys_3
              (`self.AddImageLogbookEntry` _array_element_3 (`|GetArrayItem` _values_6 _array_index_3))))))
      (else
        (`KismetSystemLibrary.PrintString` "No Save Game Found" true true (struct :`R` 1.0 :`A` 1.0))))))

(event `Key|One`
  (params (Key :type "Key Structure"))
  ;[1 1 1] Show Menu
  (:`Pressed`
    (if (`self.Grabmode`) :!label _label
      (`/Game/Gameplay/Interact/MurderBoard/Blueprint/BP_MurderBoard.DisableBoard` (`self.MurderBoard`))
      (elif (`self.LogbookVisible`)
        _
        (elif (not (`self.isPaused`))
          (bind _returnvalue (`|CreateWidget` "/Game/Menu/PauseMenuWidget.PauseMenuWidget_C"))
          (`UserWidget.AddToViewport` _returnvalue 0)
          (set `PlayerController.bShowMouseCursor` true (`GameplayStatics.GetPlayerController` 0))
          (set `self.isPaused` true)
          (`GameplayStatics.SetGamePaused` true))))))

(event `Key|Escape`
  (params (Key :type "Key Structure"))
  ;[1 1 1] Show Menu
  (:`Pressed`
    (goto _label)))

(fn `UserConstructionScript`)