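; Player pawn Blueprint that handles movement, interaction, a logbook widget and a detective view, and tracks a two-stage echo puzzle.
; While the logbook is hidden, Tick drives movement and rotation and counts echoes whose player-assigned ID matches their own.
; Matching all echoes in each ID range flags the first, then second door as activated, with only a debug print.
; Jump simply offsets the capsule upward.
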(event `self.ReceiveBeginPlay`
  (bind _returnvalue (`|CreateWidget` "/Game/UI/Logbook/BP_Logbook.BP_Logbook_C"))
  (bind _output_get (set `self.Logbook` _returnvalue))
  (`self.SetLogbook` _output_get)
  (`UserWidget.AddToViewport` _returnvalue 0))

(event `self.ReceiveTick`
  (params (DeltaSeconds :type "Float (single-precision)"))
  (if (not (`self.LogbookVisible`))
    (`self.Move` (`KismetMathLibrary.MakeVector2D` (`self.GetInputAxisValue`) (`self.GetInputAxisValue`)))
    (`self.Rotate` (`KismetMathLibrary.MakeVector2D` (`self.GetInputAxisValue`) (`self.GetInputAxisValue`)))
    (set `self.Count` 0)
    (if (`self.isFirstDoorActivated`)
      (if (not (`self.isSecondDoorActivated`))
        ;[1 1 1] For Second Door
        (for _index (range (`KismetArrayLibrary.Array_Length` (`self.EchoArray`)))
          (bind _output (`|GetArrayItem` (`self.EchoArray`) _index))
          (bind _idecho (`/Game/Gameplay/Interact/Echos/BP_Echo_Base.idEcho` _output))
          (if (> _idecho (`self.EchosForFirstDoor`))
            (if (== _idecho (`/Game/Gameplay/Interact/Echos/BP_Echo_Base.idFromPlayer` _output))
              (bind _result (`/Engine/EditorBlueprintResources/StandardMacros.IncrementInt` (`self.Count`))
                (:`  `
                  (set `self.Count` _result))))))
        (if (== (`self.Count`) (- (`self.EchosForSecondDoor`) (`self.EchosForFirstDoor`)))
          (set `self.isSecondDoorActivated` true)
          (`KismetSystemLibrary.PrintString` "Second Door Opened")))
      (else
        ;[1 1 1] For First Echos
        (for _index_2 (range (`KismetArrayLibrary.Array_Length` (`self.EchoArray`)))
          (bind _output_2 (`|GetArrayItem` (`self.EchoArray`) _index_2))
          (bind _idecho_2 (`/Game/Gameplay/Interact/Echos/BP_Echo_Base.idEcho` _output_2))
          (if (<= _idecho_2 (`self.EchosForFirstDoor`))
            (if (> _idecho_2 0)
              (if (== _idecho_2 (`/Game/Gameplay/Interact/Echos/BP_Echo_Base.idFromPlayer` _output_2))
                (bind _result_2 (`/Engine/EditorBlueprintResources/StandardMacros.IncrementInt` (`self.Count`))
                  (:`  `
                    (set `self.Count` _result_2)))))))
        (if (== (`self.Count`) (`self.EchosForFirstDoor`))
          (set `self.isFirstDoorActivated` true)
          (`KismetSystemLibrary.PrintString` "Open Door"))))))

(event `InputAction|Interact`
  (params (Key :type "Key Structure"))
  (:`Pressed`
    (`self.Interact`)))

(event `InputAction|Jump`
  (params (Key :type "Key Structure"))
  (:`Pressed`
    (`SceneComponent.K2_SetWorldLocation` (`self.Capsule`) (+ (`SceneComponent.K2_GetComponentLocation` (`self.Capsule`)) (`KismetMathLibrary.MakeVector` 0.0 0.0 (`self.JumpForce`))) false false)))

(event `InputAction|ShowHideLogbook`
  (params (Key :type "Key Structure"))
  (:`Pressed`
    (bind _output_get (set `self.LogbookVisible` (not (`self.LogbookVisible`))))
    (`self.ShowHideLogbook` _output_get)))

(event `InputAction|DetectiveView`
  (params (Key :type "Key Structure"))
  (:`Pressed`
    (`self.ActivateView`)))

(fn `UserConstructionScript`)