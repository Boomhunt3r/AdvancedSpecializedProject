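; Interactable murder board that shows four suspects and pinned Post-it hints, and fills the murder UI's suspect list.
; Interacting toggles a board camera view with mouse cursor, grab mode and hidden player mesh; Tick exits it when the player moves out of range.
; Opening spawns queued hint classes at random positions between board markers, then clears the queue.
; After a game load, spawning compares hints against the saved Post-its by name.
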(event `self.ReceiveBeginPlay`
  ;[1 1 1] Search Player ref at the beginning
  (bind _asbp_player_character (cast `/Game/Character/Player/Blueprint/BP_PlayerCharacter` (`GameplayStatics.GetPlayerCharacter` 0)))
  (set `self.PlayerRef` _asbp_player_character)
  (`self.DisableInput` (`ActorComponent.GetOwner` (`self.Camera`)) (`GameplayStatics.GetPlayerController` 0))
  (`KismetSystemLibrary.Delay` 3.0)
  ;[1 1 1] Add Display names to Array
  (set `/Game/UI/MurderBoard/BP_MurderBoardUI.AllSuspects` (`|MakeArray` (`KismetSystemLibrary.GetDisplayName` (`self.Ernest`)) (`KismetSystemLibrary.GetDisplayName` (`self.Johnathan`)) (`KismetSystemLibrary.GetDisplayName` (`self.Rose`)) (`KismetSystemLibrary.GetDisplayName` (`self.William`))) (`/Game/Character/Player/Blueprint/BP_PlayerCharacter.MurderUI` (`self.PlayerRef`))))

(event `self.Interact`
  (params (OtherActor :type "Actor Object Reference"))
  (`WidgetBlueprintLibrary.SetInputMode_GameAndUIEx` (`GameplayStatics.GetPlayerController` 0) null)
  (if (not (`self.FirstInteraction`))
    ;[1 1 1] Interact Logic
    (`SceneComponent.SetVisibility` (`self.Johnathan`) true false)
    (`SceneComponent.SetVisibility` (`self.Rose`) true false)
    (`SceneComponent.SetVisibility` (`self.William`) true false)
    (`SceneComponent.SetVisibility` (`self.Ernest`) true false)
    (set `self.FirstInteraction` true))
  (if (`self.Interacting`)
    (`self.DisableBoard`)
    (else
      (`self.EnableBoard`)
      (`self.SpawnPostIts`))))

(event `self.ReceiveTick`
  (params (DeltaSeconds :type "Float (single-precision)"))
  ;[1 1 1] Check if Player is still in Range of Board
  (if (`self.Interacting`)
    (if (>= (`KismetMathLibrary.Vector_Distance` (`SceneComponent.K2_GetComponentLocation` (`Character.Mesh` (`self.PlayerRef`))) (`SceneComponent.K2_GetComponentLocation` (`self.MurderBoard`))) 178.0)
      (`self.DisableBoard`))))

(event `SpawnPostIts`
  (bind _postithints (`self.PostItHints`))
  ;[1 1 1] Spawn Post its on Board
  (if (`/Game/Character/Player/Blueprint/BP_PlayerCharacter.isGameLoaded` (`self.PlayerRef`))
    (for _array_element _postithints
      (for _array_element_2 (`/Game/Save/BP_GameSave.PostIts` (`/Game/Character/Player/Blueprint/BP_PlayerCharacter.SaveGame` (`self.PlayerRef`)))
        (if (`KismetStringLibrary.NotEqual_StrStr` (`KismetSystemLibrary.GetDisplayName` _array_element_2) (`KismetSystemLibrary.GetClassDisplayName` _array_element))
          (bind _returnvalue (`self.CreateTransform`))
          (`|SpawnActorFromClass` _array_element (`KismetMathLibrary.MakeTransform` (.location _returnvalue)) "Undefined" "OverrideRootScale" null null)
          (set `/Game/Character/Player/Blueprint/BP_PlayerCharacter.isGameLoaded` false (`self.PlayerRef`)))))
    (`KismetArrayLibrary.Array_Clear` _postithints)
    (else
      (for _array_element_3 (`self.PostItHints`)
        (bind _returnvalue_2 (`self.CreateTransform`))
        (`|SpawnActorFromClass` _array_element_3 (`KismetMathLibrary.MakeTransform` (.location _returnvalue_2)) "Undefined" "OverrideRootScale" null null))
      (`KismetArrayLibrary.Array_Clear` (`self.PostItHints`)))))

(fn `CreateTransform`
  (returns (ReturnValue :type "Transform Structure"))
  (return (`KismetMathLibrary.MakeTransform` (`KismetMathLibrary.MakeVector` (`KismetMathLibrary.RandomFloatInRange` (.x (.location (`SceneComponent.K2_GetComponentToWorld` (`self.MurderBoard`)))) (.x (`SceneComponent.K2_GetComponentLocation` (`self.StaticMesh1`)))) (`KismetMathLibrary.RandomFloatInRange` (.y (.location (`SceneComponent.K2_GetComponentToWorld` (`self.MurderBoard`)))) (.y (`SceneComponent.K2_GetComponentLocation` (`self.StaticMesh2`)))) (.z (.location (`SceneComponent.K2_GetComponentToWorld` (`self.MurderBoard`))))) (.rotation (`SceneComponent.K2_GetComponentToWorld` (`self.MurderBoard`))) (.scale (`SceneComponent.K2_GetComponentToWorld` (`self.MurderBoard`))))))

(fn `DisableBoard`
  (bind _playerref (`self.PlayerRef`))
  (`SceneComponent.SetVisibility` (`Character.Mesh` (`self.PlayerRef`)) true false)
  (`PlayerController.SetViewTargetWithBlend` (`GameplayStatics.GetPlayerController` 0) (`GameplayStatics.GetPlayerCharacter` 0) 0.0 "VTBlend_Linear" 0.0 false)
  (set `/Game/Character/Player/Blueprint/BP_PlayerCharacter.Grabmode` false (`self.PlayerRef`))
  (set `self.Interacting` false)
  (set `PlayerController.bShowMouseCursor` false (`GameplayStatics.GetPlayerController` 0))
  (`Widget.SetVisibility` (`/Game/Character/Player/Blueprint/BP_PlayerCharacter.PostItWidget` (`self.PlayerRef`)) "Hidden")
  (`Widget.SetVisibility` (`/Game/Character/Player/Blueprint/BP_PlayerCharacter.MurderUI` _playerref) "Hidden")
  (`Widget.SetVisibility` (`/Game/Character/Player/Blueprint/BP_PlayerCharacter.PostItWidget` _playerref) "Hidden")
  (`WidgetBlueprintLibrary.SetInputMode_GameOnly` (`GameplayStatics.GetPlayerController` 0)))

(fn `EnableBoard`
  (set `/Game/Character/Player/Blueprint/BP_PlayerCharacter.Grabmode` true (`self.PlayerRef`))
  (`SceneComponent.SetVisibility` (`Character.Mesh` (`self.PlayerRef`)) false false)
  (`PlayerController.SetViewTargetWithBlend` (`GameplayStatics.GetPlayerController` 0) self 0.5 "VTBlend_Linear" 0.0 false)
  (set `self.Interacting` true)
  (set `PlayerController.bShowMouseCursor` true (`GameplayStatics.GetPlayerController` 0)))

(fn `UserConstructionScript`)