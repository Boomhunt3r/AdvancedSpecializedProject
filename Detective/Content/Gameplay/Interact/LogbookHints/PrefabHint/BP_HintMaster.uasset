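; BP_HintMaster is an interactable hint actor that adds an image entry to the player's logbook.
; Its Interact event plays an optional sound at the actor's location, then casts the interacting actor to BP_PlayerPawn and passes it the hint's ID and Texture.
; An Interacted flag makes the hint one-shot, but is set only after that cast succeeds.
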(event `self.Interact`
  (params (OtherActor :type "Actor Object Reference"))
  (bind _sound (`self.Sound`))
  (if (not (`self.Interacted`))
    (`/Engine/EditorBlueprintResources/StandardMacros.IsValid` _sound
      (:`Is Valid`
        (`GameplayStatics.PlaySoundAtLocation` _sound (`self.K2_GetActorLocation`) (struct) 1.0 1.0 0.0 null null null))
      (:`Is Not Valid`
        _))
    (bind _asbp_player_pawn (cast `/Game/Character/Player/Blueprint/BP_PlayerPawn` OtherActor))
    (`PlayerPawn.AddImageLogbookEntry` _asbp_player_pawn (`self.ID`) (`self.Texture`))
    (set `self.Interacted` true)))

(fn `UserConstructionScript`)