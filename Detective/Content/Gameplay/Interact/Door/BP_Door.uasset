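; An interactable hinged door Blueprint that swings open and closed when interacted with.
; Interact toggles the Open flag and plays the matching open or close sound at the actor's location.
; Tick rotates DoorRotateRoot in yaw by RotataionSpeed scaled by delta time, toward a quarter turn when open or back to zero when closed, without clamping at either limit.
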(event `self.Interact`
  (params (OtherActor :type "Actor Object Reference"))
  (bind _returnvalue (`self.K2_GetActorLocation`))
  (set `self.Open` (not (`self.Open`)))
  (if (`self.Open`)
    (`GameplayStatics.PlaySoundAtLocation` "/Game/Audio/Effects/Door/A_Door_Open.A_Door_Open" _returnvalue (struct) 0.7 1.0 0.0 null null null)
    (else
      (`GameplayStatics.PlaySoundAtLocation` "/Game/Audio/Effects/Door/A_Door_Close.A_Door_Close" _returnvalue (struct) 0.7 1.0 0.0 null null null))))

(event `self.ReceiveTick`
  (params (DeltaSeconds :type "Float (single-precision)"))
  (bind (_relativerotation_roll _relativerotation_pitch _relativerotation_yaw) (`KismetMathLibrary.BreakRotator` (`SceneComponent.RelativeRotation` (`self.DoorRotateRoot`))))
  (bind (_relativerotation_roll_2 _relativerotation_pitch_2 _relativerotation_yaw_2) (`KismetMathLibrary.BreakRotator` (`SceneComponent.RelativeRotation` (`self.DoorRotateRoot`))))
  (if (`self.Open`)
    (if (< _relativerotation_yaw_2 90.0)
      (`SceneComponent.K2_AddLocalRotation` (`self.DoorRotateRoot`) (`KismetMathLibrary.MakeRotator` 0.0 0.0 (* (`self.RotataionSpeed`) (`GameplayStatics.GetWorldDeltaSeconds`))) false false))
    (elif (> _relativerotation_yaw 0.0)
      (`SceneComponent.K2_AddLocalRotation` (`self.DoorRotateRoot`) (`KismetMathLibrary.MakeRotator` 0.0 0.0 (* (`self.RotataionSpeed`) (`GameplayStatics.GetWorldDeltaSeconds`) -1.0)) false false))))

(fn `UserConstructionScript`)