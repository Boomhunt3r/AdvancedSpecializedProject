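; BP_Echo_Base is an interactable Echo that the player activates, then numbers, with validity set by matching its expected ID.
; First interaction increments the pawn's ActivatedEchos, plays a sound and reveals EchoPose; later ones cycle the displayed number up to that count.
; Tick updates IsValid and, once activated, shows the pose only within ViewDistanceEcho of the player.
; GetCameraAngel yaws the number text toward the camera, but nothing here calls it.
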(event `self.ReceiveBeginPlay`
  (bind _asbp_player_pawn (cast `/Game/Character/Player/Blueprint/BP_PlayerPawn` (`GameplayStatics.GetPlayerPawn` 0)))
  (set `self.PlayerRef` _asbp_player_pawn)
  (cast `/Game/ThirdPersonBP/Blueprints/ThirdPersonGameMode` (`GameplayStatics.GetGameMode`)))

(event `self.Interact`
  (params (OtherActor :type "Actor Object Reference"))
  (if (not (`self.isActivated`))
    (bind _asbp_player_pawn (cast `/Game/Character/Player/Blueprint/BP_PlayerPawn` (`GameplayStatics.GetPlayerPawn` 0)))
    (bind _result (`/Engine/EditorBlueprintResources/StandardMacros.IncrementInt` (`/Game/Character/Player/Blueprint/BP_PlayerPawn.ActivatedEchos` _asbp_player_pawn))
      (:`  `
        (set `/Game/Character/Player/Blueprint/BP_PlayerPawn.ActivatedEchos` _result _asbp_player_pawn)
        (set `self.isActivated` true)
        (`GameplayStatics.PlaySoundAtLocation` "/Game/StarterContent/Audio/Explosion01.Explosion01" (`self.K2_GetActorLocation`) (struct) 1.0 1.0 0.0 null null null)
        (`SceneComponent.SetVisibility` (`self.EchoPose`) true true)))
    (else
      (bind _asbp_player_pawn_2 (cast `/Game/Character/Player/Blueprint/BP_PlayerPawn` (`GameplayStatics.GetPlayerPawn` 0)))
      (if (>= (`self.idFromPlayer`) (`/Game/Character/Player/Blueprint/BP_PlayerPawn.ActivatedEchos` _asbp_player_pawn_2))
        (set `self.idFromPlayer` 1)
        (else
          (set `self.idFromPlayer` (+ (`self.idFromPlayer`) 1))))
      (`TextRenderComponent.K2_SetText` (`self.idFromPlayerText`) (`KismetTextLibrary.Conv_IntToText` (`self.idFromPlayer`))))))

(event `self.ReceiveTick`
  (params (DeltaSeconds :type "Float (single-precision)"))
  (bind _echopose (`self.EchoPose`))
  (set `self.isValid` (== (`self.idEcho`) (`self.idFromPlayer`)))
  (if (`self.isActivated`)
    (if (>= (`KismetMathLibrary.VSize` (- (`SceneComponent.K2_GetComponentLocation` (`self.Clue`)) (`SceneComponent.K2_GetComponentLocation` (`PlayerPawn.Capsule` (`self.PlayerRef`))))) (`self.viewDistanceEcho`))
      (`SceneComponent.SetVisibility` _echopose false true)
      (else
        (`SceneComponent.SetVisibility` _echopose true true)))))

(fn `GetCameraAngel`
  (`SceneComponent.K2_SetRelativeRotation` (`self.idFromPlayerText`) (`KismetMathLibrary.Conv_VectorToRotator` (`KismetMathLibrary.Normal` (* (- (`PlayerCameraManager.GetCameraLocation` (`GameplayStatics.GetPlayerCameraManager` 0)) (`self.K2_GetActorLocation`)) (1.0 1.0 0.0)))) false false))

(fn `UserConstructionScript`)