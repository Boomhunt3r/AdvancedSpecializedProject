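; BP_Echo_Fence is an interactable echo that reveals a fence mesh once the player activates it.
; The first interaction sets a one-way activated flag, plays an explosion sound and shows EchoFence.
; Once activated, Tick compares the distance from the Placeholder component to the player capsule, cached on BeginPlay, against ViewDistanceEcho, showing the fence only within that range.
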(event `self.Interact`
  (params (OtherActor :type "Actor Object Reference"))
  (if (not (`self.isActivated`))
    (set `self.isActivated` true)
    (`GameplayStatics.PlaySoundAtLocation` "/Game/StarterContent/Audio/Explosion01.Explosion01" (`self.K2_GetActorLocation`) (struct) 1.0 1.0 0.0 null null null)
    (`SceneComponent.SetVisibility` (`self.Echo_Fence`) true false)))

(event `self.ReceiveTick`
  (params (DeltaSeconds :type "Float (single-precision)"))
  (bind _echo_fence (`self.Echo_Fence`))
  (if (`self.isActivated`)
    (if (>= (`KismetMathLibrary.VSize` (- (`SceneComponent.K2_GetComponentLocation` (`self.Placeholder`)) (`SceneComponent.K2_GetComponentLocation` (`PlayerPawn.Capsule` (`self.PlayerRef`))))) (`self.viewDistanceEcho`))
      (`SceneComponent.SetVisibility` _echo_fence false false)
      (else
        (`SceneComponent.SetVisibility` _echo_fence true false)))))

(event `self.ReceiveBeginPlay`
  (bind _asbp_player_pawn (cast `/Game/Character/Player/BP_PlayerPawn` (`GameplayStatics.GetPlayerPawn` 0)))
  (set `self.PlayerRef` _asbp_player_pawn))

(fn `UserConstructionScript`)