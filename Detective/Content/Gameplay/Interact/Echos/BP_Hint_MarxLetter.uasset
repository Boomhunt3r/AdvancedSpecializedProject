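; BP_Hint_MarxLetter is an interactable hint that shows and hides a Marx letter on screen.
; BeginPlay creates the Marx widget hidden in the viewport (stored as LetterThatcher despite its name) and caches the player character.
; Interact toggles its visibility, notifies the widget, and records the player mesh location on opening.
; Tick closes the letter as soon as that location changes, so any movement dismisses it.
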(event `self.ReceiveBeginPlay`
  (`parent.ReceiveBeginPlay`)
  (bind _returnvalue (`|CreateWidget` "/Game/Gameplay/Interact/Echos/Widget_Marx.Widget_Marx_C"))
  (bind _output_get (set `self.Letter_Thatcher` _returnvalue))
  (`UserWidget.AddToViewport` _output_get 0)
  (`Widget.SetVisibility` _output_get "Hidden")
  (bind _asbp_player_character (cast `/Game/Character/Player/Blueprint/BP_PlayerCharacter` (`GameplayStatics.GetPlayerCharacter` 0)))
  (set `self.Player Ref` _asbp_player_character))

(event `self.ReceiveTick`
  (params (DeltaSeconds :type "Float (single-precision)"))
  (bind _letter_thatcher (`self.Letter_Thatcher`))
  (`parent.ReceiveTick` DeltaSeconds)
  (if (`self.WidgetActive`)
    (if (!= (`self.Location`) (`SceneComponent.K2_GetComponentLocation` (`Character.Mesh` (`self.Player Ref`))))
      (`Widget.SetVisibility` _letter_thatcher "Hidden")
      (set `self.WidgetActive` false)
      (`/Game/Gameplay/Interact/Echos/Widget_Marx.WidgetMarxDeactive` _letter_thatcher))))

(event `self.Interact`
  (params (OtherActor :type "Actor Object Reference"))
  (bind _letter_thatcher (`self.Letter_Thatcher`))
  (`parent.Interact` null)
  (if (`self.WidgetActive`)
    (`Widget.SetVisibility` _letter_thatcher "Hidden")
    (set `self.WidgetActive` false)
    (`/Game/Gameplay/Interact/Echos/Widget_Marx.WidgetMarxDeactive` _letter_thatcher)
    (else
      (`Widget.SetVisibility` _letter_thatcher "Visible")
      (set `self.WidgetActive` true)
      (`/Game/Gameplay/Interact/Echos/Widget_Marx.WidgetMarxActive` _letter_thatcher)
      (set `self.Location` (`SceneComponent.K2_GetComponentLocation` (`Character.Mesh` (`self.Player Ref`)))))))

(fn `UserConstructionScript`
  (`parent.UserConstructionScript`))