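; Base Blueprint for an interactable hint ("Echo") that feeds clues to the player's logbook and the murder board.
; On BeginPlay it registers in the player pawn's EchoArray and finds BP_MurderBoard.
; The first interaction flags a HUD message, adds its post-it and logbook page, increments the activated Echo count and plays a success sound.
; Older ID-cycling, door-check and distance-visibility logic remains disconnected, and Tick is empty.
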(event `self.ReceiveTick`
  (params (DeltaSeconds :type "Float (single-precision)"))
  ;[1 1 1] Distance between Echo and Player to set Echo Visibility
)

(event `self.ReceiveBeginPlay`
  ;[1 1 1] Create Echo Array
  (bind _asbp_player_pawn (cast `/Game/Character/Player/Blueprint/BP_PlayerPawn` (`GameplayStatics.GetPlayerPawn` 0)))
  (set `self.PlayerRef` _asbp_player_pawn)
  (cast `/Game/ThirdPersonBP/Blueprints/ThirdPersonGameMode` (`GameplayStatics.GetGameMode`))
  (`KismetArrayLibrary.Array_Add` (`/Game/Character/Player/Blueprint/BP_PlayerPawn.EchoArray` (`self.PlayerRef`)) self)
  (bind _returnvalue (`GameplayStatics.GetActorOfClass` "/Game/Gameplay/Interact/MurderBoard/Blueprint/BP_MurderBoard.BP_MurderBoard_C"))
  (set `self.BoardRef` _returnvalue))

(event `self.Interact`
  (params (OtherActor :type "Actor Object Reference"))
  (if (not (`self.isActivated`))
    (set `/Game/UI/MainHUD/Widget_MainHUD.ShowMessage` true (`/Game/Character/Player/Blueprint/BP_PlayerPawn.MainHUD` (`self.PlayerRef`)))
    ;[1 1 1] Make Pose and ID Visioble after Interaction
    (`KismetArrayLibrary.Array_Add` (`/Game/Gameplay/Interact/MurderBoard/Blueprint/BP_MurderBoard.PostItHints` (`self.BoardRef`)) (`self.PostIt`))
    (bind _asbp_player_pawn (cast `/Game/Character/Player/Blueprint/BP_PlayerPawn` (`GameplayStatics.GetPlayerPawn` 0)))
    (`PlayerPawn.AddImageLogbookEntry` _asbp_player_pawn (`self.ID`) (`self.LogBook_Page`))
    (bind _result (`/Engine/EditorBlueprintResources/StandardMacros.IncrementInt` (`/Game/Character/Player/Blueprint/BP_PlayerPawn.ActivatedEchos` _asbp_player_pawn))
      (:`  `
        (set `/Game/Character/Player/Blueprint/BP_PlayerPawn.ActivatedEchos` _result _asbp_player_pawn)
        (set `self.isActivated` true)
        (`GameplayStatics.PlaySoundAtLocation` "/Game/Audio/Effects/A_Success.A_Success" (`self.K2_GetActorLocation`) (struct) 0.2 1.0 0.0 null null null)))))

(fn `GetCameraAngel`
  (`SceneComponent.K2_SetRelativeRotation` (`self.idFromPlayerText`) (`KismetMathLibrary.Conv_VectorToRotator` (`KismetMathLibrary.Normal` (* (- (`PlayerCameraManager.GetCameraLocation` (`GameplayStatics.GetPlayerCameraManager` 0)) (`self.K2_GetActorLocation`)) (1.0 1.0 0.0)))) false false))

(fn `UserConstructionScript`)