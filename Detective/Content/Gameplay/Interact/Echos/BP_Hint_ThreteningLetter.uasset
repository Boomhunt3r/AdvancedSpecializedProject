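; BP_Hint_ThreteningLetter is an interactable hint that shows a Chadwick letter widget on screen.
; BeginPlay creates the widget hidden in the viewport and caches the player character.
; Interact toggles the letter's visibility, calls its activate or deactivate event, and records the player mesh location on opening.
; While the letter is open, Tick compares that saved location to the current one and closes the letter once the player moves.
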(event `self.ReceiveBeginPlay`
  (`parent.ReceiveBeginPlay`)
  (bind _returnvalue (`|CreateWidget` "/Game/Gameplay/Interact/Echos/Widget_Chadwick.Widget_Chadwick_C"))
  (bind _output_get (set `self.LetterChadwick` _returnvalue))
  (`UserWidget.AddToViewport` _output_get 0)
  (`Widget.SetVisibility` _output_get "Hidden")
  (bind _asbp_player_character (cast `/Game/Character/Player/Blueprint/BP_PlayerCharacter` (`GameplayStatics.GetPlayerCharacter` 0)))
  (set `self.Player Ref` _asbp_player_character))

(event `self.ReceiveTick`
  (params (DeltaSeconds :type "Float (single-precision)"))
  (bind _letterchadwick (`self.LetterChadwick`))
  (`parent.ReceiveTick` DeltaSeconds)
  (if (`self.WidgetActive`)
    (if (!= (`self.Location`) (`SceneComponent.K2_GetComponentLocation` (`Character.Mesh` (`self.Player Ref`))))
      (`Widget.SetVisibility` _letterchadwick "Hidden")
      (set `self.WidgetActive` false)
      (`/Game/Gameplay/Interact/Echos/Widget_Chadwick.WidgetChadDeactive` _letterchadwick))))

(event `self.Interact`
  (params (OtherActor :type "Actor Object Reference"))
  (bind _letterchadwick (`self.LetterChadwick`))
  (`parent.Interact` null)
  (if (`self.WidgetActive`)
    (`Widget.SetVisibility` _letterchadwick "Hidden")
    (set `self.WidgetActive` false)
    (`/Game/Gameplay/Interact/Echos/Widget_Chadwick.WidgetChadDeactive` _letterchadwick)
    (else
      (`Widget.SetVisibility` _letterchadwick "Visible")
      (set `self.WidgetActive` true)
      (`/Game/Gameplay/Interact/Echos/Widget_Chadwick.WidgetChadActive` _letterchadwick)
      (`/Game/Gameplay/Interact/Echos/Widget_Chadwick.WidgetChadActive` _letterchadwick)
      (set `self.Location` (`SceneComponent.K2_GetComponentLocation` (`Character.Mesh` (`self.Player Ref`)))))))

(fn `UserConstructionScript`
  (`parent.UserConstructionScript`))