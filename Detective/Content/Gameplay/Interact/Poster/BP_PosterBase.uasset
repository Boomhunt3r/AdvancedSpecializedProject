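; Base interactable poster actor that shows its texture in an on-screen PosterBase widget.
; BeginPlay creates the widget, adds it hidden to the viewport, assigns the texture and caches the BP_PlayerPawn reference.
; Interact toggles the widget's visibility and, when showing it, records the player capsule's location.
; Tick hides the poster once the player moves from that recorded location.
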(event `self.ReceiveBeginPlay`
  (bind _returnvalue (`|CreateWidget` "/Game/Gameplay/Interact/Poster/PosterBase.PosterBase_C"))
  (set `self.Widget` _returnvalue)
  (`UserWidget.AddToViewport` _returnvalue 0)
  (`Widget.SetVisibility` (`self.Widget`) "Hidden")
  (`Image.SetBrushFromTexture` (`/Game/Gameplay/Interact/Poster/PosterBase.PosterImage` (`self.Widget`)) (`self.Texture `) false)
  (bind _asbp_player_pawn (cast `/Game/Character/Player/Blueprint/BP_PlayerPawn` (`GameplayStatics.GetPlayerPawn` 0)))
  (set `self.Player Ref` _asbp_player_pawn))

(event `self.ReceiveTick`
  (params (DeltaSeconds :type "Float (single-precision)"))
  (if (`self.Isactivated`)
    (if (!= (`self.Location`) (`SceneComponent.K2_GetComponentLocation` (`PlayerPawn.Capsule` (`self.Player Ref`))))
      (`Widget.SetVisibility` (`self.Widget`) "Hidden")
      (set `self.Isactivated` false))))

(event `self.Interact`
  (params (OtherActor :type "Actor Object Reference"))
  (if (`self.Isactivated`)
    (`Widget.SetVisibility` (`self.Widget`) "Hidden")
    (set `self.Isactivated` false)
    (else
      (`Widget.SetVisibility` (`self.Widget`) "Visible")
      (set `self.Isactivated` true)
      (set `self.Location` (`SceneComponent.K2_GetComponentLocation` (`PlayerPawn.Capsule` (`self.Player Ref`)))))))

(fn `UserConstructionScript`)